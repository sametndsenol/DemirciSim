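; EmptyBucket is an actor Blueprint for an empty bucket that the first-person character can pick up.
; Interact finds the FirstPersonCharacter and attaches to its El1 socket, snapping location and keeping relative rotation and scale.
; FKEY only prints a debug message.
; Mesh swapping and the KovaEldeMi held-bucket flag sit in unconnected nodes that never run.
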(fn `F-KEY`
  (returns (`Did f` :type Boolean))
  (locals (NewLocalVar_0 :type "Array of StaticMesh Object Reference"))
  (`KismetSystemLibrary.PrintString` "Hello")
  (return false))

(fn `Interact`
  (returns (`did interact` :type Boolean))
  (bind _returnvalue (`GameplayStatics.GetActorOfClass` "/Game/Blueprint/FirstPersonCharacter.FirstPersonCharacter_C"))
  (`self.K2_AttachToActor` _returnvalue "El1" "SnapToTarget" "KeepRelative" "KeepRelative")
  (return false))

(fn `UserConstructionScript`)