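; Carryable bucket actor that fills with iron or coal in up to three steps, showing each step by swapping its static mesh.
; Interact snaps it to the FirstPersonCharacter's palm socket and sets BucketOnHand, which gates both fill events.
; ChangeMeshIron and ChangeMeshCoal apply the current MeshCounter mesh, then advance fullness and set the next index.
; Content type is recorded on the first fill and not checked afterwards; FKEY is an inactive stub.
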(event `ChangeMeshIron`
  (bind _cube (`self.Cube`))
  (bind _output (`|GetArrayItem` (`self.meshes`) (`self.MeshCounter`)))
  (if (`self.BucketOnHand`)
    (if (== (`self.BucketFullness`) 0)
      (`StaticMeshComponent.SetStaticMesh` _cube _output)
      (set `self.BucketFullness` 1)
      (set `self.MeshCounter` 4)
      (set `self.BucketContent` "Iron")
      (elif (== (`self.BucketFullness`) 1)
        (`StaticMeshComponent.SetStaticMesh` _cube _output)
        (set `self.BucketFullness` 2)
        (set `self.MeshCounter` 5)
        (elif (== (`self.BucketFullness`) 2)
          (`StaticMeshComponent.SetStaticMesh` _cube _output)
          (set `self.BucketFullness` 3)
          (set `self.MeshCounter` 6))))))

(event `ChangeMeshCoal`
  (bind _cube (`self.Cube`))
  (bind _output (`|GetArrayItem` (`self.meshes`) (`self.MeshCounter`)))
  (if (`self.BucketOnHand`)
    (if (== (`self.BucketFullness`) 0)
      (`StaticMeshComponent.SetStaticMesh` _cube _output)
      (set `self.BucketFullness` 1)
      (set `self.MeshCounter` 2)
      (set `self.BucketContent` "Coal")
      (elif (== (`self.BucketFullness`) 1)
        (`StaticMeshComponent.SetStaticMesh` _cube _output)
        (set `self.BucketFullness` 2)
        (set `self.MeshCounter` 3)
        (elif (== (`self.BucketFullness`) 2)
          (`StaticMeshComponent.SetStaticMesh` _cube _output)
          (set `self.BucketFullness` 3)
          (set `self.MeshCounter` 3))))))

(fn `F-KEY`
  (returns (`Did f` :type Boolean))
  (return false))

(fn `Interact`
  (returns (`did interact` :type Boolean))
  (bind _returnvalue (`GameplayStatics.GetActorOfClass` "/Game/Blueprint/FirstPersonCharacter.FirstPersonCharacter_C"))
  (`self.K2_AttachToActor` _returnvalue "palm_04_LSocket" "SnapToTarget" "KeepRelative" "KeepRelative")
  (set `self.BucketOnHand` true)
  (return false))

(fn `UserConstructionScript`)