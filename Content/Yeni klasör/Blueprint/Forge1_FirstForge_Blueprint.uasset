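; Forge Blueprint for the first forge, which can be filled with coal from a bucket.
; Its F-KEY function checks that the referenced Bucket holds Coal at a fullness of three, then makes the forge's Cube visible.
; It then empties the bucket directly, swapping its mesh to the empty version and clearing its content, fullness and mesh counter.
; The event graph and construction script contain no logic.
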(fn `F-KEY`
  (returns (`Did f` :type Boolean))
  (bind _bucket (`self.Bucket`))
  (if (`KismetStringLibrary.EqualEqual_StrStr` (`/Game/Blueprint/mesh-degistirme.BucketContent` (`self.Bucket`)) "Coal")
    (if (== (`/Game/Blueprint/mesh-degistirme.BucketFullness` (`self.Bucket`)) 3)
      (`SceneComponent.SetVisibility` (`self.Cube`) true false)
      (`StaticMeshComponent.SetStaticMesh` (`/Game/Blueprint/mesh-degistirme.Cube` (`self.Bucket`)) "/Game/Geometry/Meshes/EmptyBucket.EmptyBucket")
      (set `/Game/Blueprint/mesh-degistirme.BucketFullness` 0 _bucket)
      (set `/Game/Blueprint/mesh-degistirme.MeshCounter` 0 _bucket)
      (set `/Game/Blueprint/mesh-degistirme.BucketContent` "" _bucket)
      (return false))))

(fn `UserConstructionScript`)