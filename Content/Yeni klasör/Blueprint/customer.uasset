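; Customer actor that walks a short scripted path on spawn and shows a UI widget when interacted with.
; On BeginPlay it waits briefly, then slides its Cube component through two relative positions in sequence using MoveComponentTo.
; Interact creates a NewWidgetBlueprint for the first player controller, stores it and adds it to the viewport.
; The F-KEY function hides that stored widget rather than removing it.
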(event `self.ReceiveBeginPlay`
  (`KismetSystemLibrary.Delay` 2.0)
  (`KismetSystemLibrary.MoveComponentTo` (`self.Cube`) (0.0 -400.0 0.0) (struct) false false 1.0)
  (`KismetSystemLibrary.MoveComponentTo` (`self.Cube`) (-400.0 -400.0 0.0) (struct) false false 1.0))

(fn `F-KEY`
  (returns (`Did f` :type Boolean))
  (`Widget.SetVisibility` (`self.NewVar_0`) "Hidden")
  (return false))

(fn `Interact`
  (returns (`did interact` :type Boolean))
  (bind _returnvalue (`|CreateWidget` "/Game/Blueprint/NewWidgetBlueprint.NewWidgetBlueprint_C" (`GameplayStatics.GetPlayerController` 0)))
  (bind _output_get (set `self.NewVar_0` _returnvalue))
  (`UserWidget.AddToViewport` _output_get 0)
  (return false))

(fn `UserConstructionScript`)