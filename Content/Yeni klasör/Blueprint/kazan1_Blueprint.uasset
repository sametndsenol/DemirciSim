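; Interactable actor (kazan, "cauldron") that tilts in pitch while an interaction is active.
; Interact and Etkileşim2 set and clear the IsEPressed flag that Tick reads.
; While set, Tick applies a frame-rate-scaled local pitch rotation as long as pitch is within a limit; otherwise RInterpTo slowly eases the actor toward a fixed rest rotation.
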(event `self.ReceiveTick`
  (params (DeltaSeconds :type "Float (single-precision)"))
  (if (`self.is e pressed`)
    (if (<= (.pitch (`self.K2_GetActorRotation`)) 60.0)
      (`self.K2_AddActorLocalRotation` (* (`KismetMathLibrary.MakeRotator` 0.0 180.0) DeltaSeconds)))
    (else
      (`self.K2_SetActorRotation` (`KismetMathLibrary.RInterpTo` (`self.K2_GetActorRotation`) (struct :`Yaw` 60.0) (`GameplayStatics.GetWorldDeltaSeconds`) 0.5)))))

(fn `Etkileşim 2`
  (returns (NewParam :type Boolean))
  (set `self.is e pressed` false)
  (return false))

(fn `Interact`
  (returns (`did interact` :type Boolean))
  (set `self.is e pressed` true)
  (return false))

(fn `UserConstructionScript`)